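; Base projectile Blueprint, named as a parent class, that damages enemies it overlaps.
; The construction script sets the movement component's initial and max speed from ProjectileSpeed, and BeginPlay rotates the actor to face its velocity.
; On overlap with an actor whose first tag is Enemy, it subtracts Damage from a living BP_Enemy's Health, calls HealthCheck, then destroys itself even if that enemy's health was already depleted.
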(event `self.ReceiveBeginPlay`
  (bind _returnvalue (`self.K2_GetActorLocation`))
  (`self.K2_SetActorRotation` (`KismetMathLibrary.FindLookAtRotation` _returnvalue (+ _returnvalue (`self.GetVelocity`)))))

(event `self.ReceiveActorBeginOverlap`
  (params (OtherActor :type "Actor Object Reference"))
  (bind _asbp_enemy (cast `/Game/Blueprints/BP_Enemy` OtherActor :!pure true))
  (switch `name` (`|GetArrayItem` (`Actor.Tags` OtherActor))
    (:`Enemy`
      (if (> (`/Game/Blueprints/BP_Enemy.Health` _asbp_enemy) 0.0)
        (set `/Game/Blueprints/BP_Enemy.Health` (- (`/Game/Blueprints/BP_Enemy.Health` _asbp_enemy) (`self.Damage`)) _asbp_enemy)
        (`/Game/Blueprints/BP_Enemy.HealthCheck` _asbp_enemy))
      (`self.K2_DestroyActor`))))

(fn `UserConstructionScript`
  (bind _projectilemovement (`self.ProjectileMovement`))
  (bind _projectile_speed (`self.Projectile_Speed`))
  (set `ProjectileMovementComponent.InitialSpeed` _projectile_speed _projectilemovement)
  (set `ProjectileMovementComponent.MaxSpeed` _projectile_speed _projectilemovement))