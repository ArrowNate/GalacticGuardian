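; Game mode that runs data-driven enemy waves, starting shortly after BeginPlay.
; SpawnLoop reads the Data_Gameplay row named by its counter and spawns that wave's enemies, taking class, location, health, score, movement and shooting settings from per-index arrays.
; After the row's sequence duration, it clears the spawned list and calls itself for the next row.
; A missing row ends the loop, with a winning screen still to be added.
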(event `self.ReceiveBeginPlay`
  (`KismetSystemLibrary.Delay` 1.0)
  (`self.Spawn Loop`))

(event `Spawn Loop`
  (bind _returnvalue (`|GetDataTableRow` "/Game/Blueprints/Data_Gameplay.Data_Gameplay" (`KismetStringLibrary.Conv_StringToName` (`KismetStringLibrary.Conv_IntToString` (`self.Spawn_Loop_Counter`)))) ; Need To Come Back to Row Not Found to Put a Winning Screen
    (:`then`
      (bind _output_get (set `self.Current_Row_Data` _returnvalue))
      (bind (_sequence _sequenceduration _scene _enemycount _actor _locations _movements _health _movespeedmultiplier _xymultiplier _velocity _canshoot _firerate _projectile _scoregive) (break `/Game/Blueprints/Struct_Gameplay` _output_get))
      (set `self.Spawn_Delay` _sequenceduration)
      (set `self.Scene` _scene)
      (for _index (range _enemycount)
        (bind (_x _y) (`KismetMathLibrary.BreakVector2D` (`self.Get_Array_Element` _xymultiplier _index)))
        (bind _returnvalue_2 (`|SpawnActorFromClass` (`|GetArrayItem` (`self.Enemy_Classes`) (`self.Get_Array_Element` _actor _index)) (`KismetMathLibrary.MakeTransform` (`self.Get_Array_Element` _locations _index)) "Undefined" "OverrideRootScale" null (`self.Get_Array_Element` _health _index) (`self.Get_Array_Element` _scoregive _index) (`self.Get_Array_Element` _movements _index) (`self.Get_Array_Element` _movespeedmultiplier _index) _x _y (`self.Get_Array_Element` _velocity _index) (`self.Get_Array_Element` _canshoot _index) (`self.Get_Array_Element` _firerate _index) null null))
        (`KismetArrayLibrary.Array_AddUnique` (`self.Enemies_Spawned`) _returnvalue_2))
      (bind _result (`/Engine/EditorBlueprintResources/StandardMacros.IncrementInt` (`self.Spawn_Loop_Counter`))
        (:`  `
          (set `self.Spawn_Loop_Counter` _result)
          (`KismetSystemLibrary.RetriggerableDelay` (`self.Spawn_Delay`))
          (`KismetArrayLibrary.Array_Clear` (`self.Enemies_Spawned`))
          (`self.Spawn Loop`))))))

(fn `UserConstructionScript`)