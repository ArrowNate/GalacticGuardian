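; Player pawn Blueprint that handles movement, firing, death and the pause menu.
; Up and Right axis inputs move it relative to control yaw, while Fire spawns a projectile at the Scene component with a sound unless dead.
; Death, ignored while invincible, shows the game-over widget, plays an explosion sound and pauses after a brief delay.
; Pause Game toggles a cached pause widget, game pause and input mode, leaving the cursor visible either way.
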(event `InputAxis|Up`
  (params (AxisValue :type "Float (single-precision)"))
  ;[1 1 1] Handle Player Movement
  (`self.AddMovementInput` (`KismetMathLibrary.GetForwardVector` (`KismetMathLibrary.MakeRotator` 0.0 0.0 (.yaw (`self.GetControlRotation`)))) AxisValue))

(event `InputAxis|Right`
  (params (AxisValue :type "Float (single-precision)"))
  ;[1 1 1] Handle Player Movement
  (`self.AddMovementInput` (`KismetMathLibrary.GetRightVector` (`KismetMathLibrary.MakeRotator` 0.0 0.0 (.yaw (`self.GetControlRotation`)))) AxisValue))

(event `Death`
  ;[1 1 1] Handle Player Death
  (if (not (`self.Invincibile`))
    (set `self.Dead` true)
    (bind _returnvalue (`|CreateWidget` "/Game/Blueprints/BP_Gameover.BP_Gameover_C"))
    (`UserWidget.AddToViewport` _returnvalue 0)
    (`GameplayStatics.PlaySound2D` "/Game/StarterContent/Audio/Explosion_Cue.Explosion_Cue" 1.0 1.0 0.0 null null)
    (`KismetSystemLibrary.Delay` 0.2)
    (`GameplayStatics.SetGamePaused` true)))

(event `InputAction|Pause Game` :paused true
  (params (Key :type "Key Structure"))
  (bind _returnvalue (`GameplayStatics.GetPlayerController` 0))
  (bind _pause_menu_reference (`self.Pause Menu Reference`))
  ;[1 1 1] Handle Pause Game
  (:`Pressed`
    (`/Engine/EditorBlueprintResources/StandardMacros.IsValid` null
      (:`Is Valid`
        _)
      (:`Is Not Valid`
        (bind _returnvalue_2 (`|CreateWidget` "/Game/Blueprints/BP_Pause.BP_Pause_C"))
        (set `self.Pause Menu Reference` _returnvalue_2)))
    (if (`GameplayStatics.IsGamePaused`)
      (`Widget.RemoveFromParent` _pause_menu_reference)
      (`GameplayStatics.SetGamePaused` false)
      (set `PlayerController.bShowMouseCursor` true _returnvalue)
      (`WidgetBlueprintLibrary.SetInputMode_GameOnly` _returnvalue)
      (else
        (`UserWidget.AddToViewport` _pause_menu_reference 0)
        (`GameplayStatics.SetGamePaused` true)
        (set `PlayerController.bShowMouseCursor` true _returnvalue)
        (`WidgetBlueprintLibrary.SetInputMode_GameAndUIEx` _returnvalue _pause_menu_reference "DoNotLock" false)))))

(event `InputAction|Fire`
  (params (Key :type "Key Structure"))
  ;[1 1 1] Handle Fire
  (:`Pressed`
    (if (not (`self.Dead`))
      (`|SpawnActorFromClass` (`self.Projectile`) (`SceneComponent.K2_GetComponentToWorld` (`self.Scene`)) "Undefined" "OverrideRootScale" null 3000.0 50.0 null)
      (`GameplayStatics.PlaySound2D` "/Engine/VREditor/Sounds/UI/Teleport_Committed.Teleport_Committed" 1.0 1.0 0.0 null null))))

(fn `UserConstructionScript`)